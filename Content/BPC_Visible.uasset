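; BPC_Visible is a component that tracks whether its owning actor is out of the player's sight.
; It finds BP_FirstPersonCharacter on BeginPlay and stores it as Player.
; Each tick it sets OutOfSight when a dot product of camera forward and the owner-to-camera vector is positive, meaning the owner is behind the camera.
; The test is a plain half-space check, ignoring field of view and occlusion.
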(event `self.ReceiveBeginPlay`
  (bind _returnvalue (`GameplayStatics.GetActorOfClass` "/Game/FirstPerson/Blueprints/BP_FirstPersonCharacter.BP_FirstPersonCharacter_C"))
  (set `self.Player` _returnvalue))

(event `self.ReceiveTick`
  (params (DeltaSeconds :type "Float (single-precision)"))
  (bind _firstpersoncamera (`/Game/FirstPerson/Blueprints/BP_FirstPersonCharacter.FirstPersonCamera` (`self.Player`)))
  (set `self.OutOfSight` (> (`KismetMathLibrary.Dot_VectorVector` (`SceneComponent.GetForwardVector` _firstpersoncamera) (- (`SceneComponent.K2_GetComponentLocation` _firstpersoncamera) (`Actor.K2_GetActorLocation` (`self.GetOwner`)))) 0.0)))