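; Washing machine that takes and destroys the towel the player is holding when interacted with.
; Once no towels remain, it spawns toilet paper, resets the curtain and calls Toggle.
; Toggle alternates between opening the door with a light fade-in and widget timer, and reversing that while stopping the timer.
; A separate END event plays a closing animation; both timelines use power-curve easing on door rotation.
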(event `/Game/FirstPerson/Blueprints/BPI_Interact.InteractedWith`
  (params (Player :type "/Game/FirstPerson/Blueprints/BP_FirstPersonCharacter Object Reference"))
  (bind _asbp_towel (cast `/Game/Towel/BP_Towel` (`/Game/FirstPerson/Blueprints/BP_FirstPersonCharacter.GrabbedActor` Player)))
  (set `/Game/FirstPerson/Blueprints/BP_FirstPersonCharacter.GrabbedActor` null Player)
  (`GameplayStatics.PlaySoundAtLocation` "/Game/Sound/SW_TowelDrop.SW_TowelDrop" (`self.K2_GetActorLocation` _asbp_towel) (struct) 1.0 1.0 0.0 null null null null)
  (`self.K2_DestroyActor` _asbp_towel)
  (bind _outactors (`GameplayStatics.GetAllActorsOfClass` "/Game/Towel/BP_Towel.BP_Towel_C"))
  (if (`KismetArrayLibrary.Array_IsEmpty` _outactors)
    (`|SpawnActorFromClass` "/Game/Papertoilet/BP_ToiletPaper.BP_ToiletPaper_C" (`KismetMathLibrary.MakeTransform` (110.70447 113.392416 69.821649) (struct :`Yaw` 90.0)) "Undefined" "MultiplyWithRoot" null null)
    (bind _returnvalue (`GameplayStatics.GetActorOfClass` "/Game/Curtain/BP_Curtain.BP_Curtain_C"))
    (`/Game/Curtain/BP_Curtain.Reset` _returnvalue)
    (`self.Toggle`)))

(event `Toggle`
  (`/Engine/EditorBlueprintResources/StandardMacros.FlipFlop`
    (:`A`
      (bind _returnvalue (`|CreateWidget` "/Game/WashingMachine/WBP_Timer.WBP_Timer_C"))
      (bind _output_get (set `self.Timer` _returnvalue))
      (`/Game/WashingMachine/WBP_Timer.StartTimer` _returnvalue)
      (`/Game/WashingMachine/WBP_Timer.StartTimer` _output_get)
      (`WidgetComponent.SetWidget` (`self.Widget`) _returnvalue)
      (`GameplayStatics.PlaySoundAtLocation` "/Game/Sound/SW_Open.SW_Open" (`self.K2_GetActorLocation`) (struct) 1.0 1.0 0.0 null null null null)
      (bind (_direction _alpha) (`Timeline|Timeline` :!label _label)
        (:`Update`
          (`LightComponent.SetIntensity` (`self.PointLight`) (`KismetMathLibrary.Lerp` 0.0 0.1 _alpha))
          (`SceneComponent.K2_SetRelativeRotation` (`self.WashingMachine_xyj_gaizi`) (`KismetMathLibrary.RLerp` (struct :`Yaw` 115.0) (struct) (`KismetMathLibrary.MultiplyMultiply_FloatFloat` (- 1.0 _alpha) 4.0) true) false false))))
    (:`B`
      (`/Game/WashingMachine/WBP_Timer.StopTimer` (`self.Timer`))
      (`GameplayStatics.PlaySoundAtLocation` "/Game/Sound/SW_Close.SW_Close" (`self.K2_GetActorLocation`) (struct) 1.0 1.0 0.0 null null null null)
      (goto _label :!via `Reverse`))))

(event `END`
  (`GameplayStatics.PlaySoundAtLocation` "/Game/Sound/SW_Close.SW_Close" (`self.K2_GetActorLocation`) (struct) 1.0 1.0 0.0 null null null null)
  (bind (_direction _alpha) (`Timeline|Timeline_0` :!via `PlayFromStart`)
    (:`Update`
      (`SceneComponent.K2_SetRelativeRotation` (`self.WashingMachine_xyj_gaizi`) (`KismetMathLibrary.RLerp` (struct :`Yaw` 115.0) (struct) (`KismetMathLibrary.MultiplyMultiply_FloatFloat` _alpha 4.0) true) false false))))

(fn `UserConstructionScript`)