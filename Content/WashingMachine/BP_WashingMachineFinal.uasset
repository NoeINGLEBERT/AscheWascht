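; Final washing machine that takes a BP_FinalTowel from the player and runs a scripted, apparently end-of-game sequence.
; Interaction destroys the towel, disables player collision and Start, teleports them to the child actor, then after delays toggles the lid and fades in fire audio as three spotlight cones widen.
; Toggle flip-flops an eased lid timeline with open/close sounds; the point light fades in on BeginPlay and dims as the lid closes.
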(event `self.ReceiveBeginPlay`
  (bind (_direction _alpha) (`Timeline|Timeline_0` :!via `PlayFromStart`)
    (:`Update`
      (`LightComponent.SetIntensity` (`self.PointLight1`) (`KismetMathLibrary.Lerp` 0.0 2.0 _alpha)))))

(event `/Game/FirstPerson/Blueprints/BPI_Interact.InteractedWith`
  (params (Player :type "/Game/FirstPerson/Blueprints/BP_FirstPersonCharacter Object Reference"))
  (bind _asbp_final_towel (cast `/Game/Towel/BP_FinalTowel` (`/Game/FirstPerson/Blueprints/BP_FirstPersonCharacter.GrabbedActor` Player)))
  (set `/Game/FirstPerson/Blueprints/BP_FirstPersonCharacter.GrabbedActor` null Player)
  (`self.K2_DestroyActor` _asbp_final_towel)
  (`PrimitiveComponent.SetCollisionEnabled` (`Character.CapsuleComponent` Player) "NoCollision")
  (`self.K2_SetActorLocation` Player (`SceneComponent.K2_GetComponentLocation` (`self.ChildActor`)) false false)
  (set `/Game/FirstPerson/Blueprints/BP_FirstPersonCharacter.Start` false Player)
  (`KismetSystemLibrary.Delay` 2.0)
  (`self.Toggle`)
  (`KismetSystemLibrary.Delay` 2.0)
  (bind _returnvalue (`GameplayStatics.SpawnSoundAtLocation` "/Game/Sound/SW_Fire.SW_Fire" (`self.K2_GetActorLocation`) (struct) 1.0 1.0 0.0 null null false))
  (`AudioComponent.SetVolumeMultiplier` _returnvalue 0.0)
  (bind (_direction _alpha) (`Timeline|Timeline_1` :!via `PlayFromStart`)
    (:`Update`
      (bind _returnvalue_2 (`KismetMathLibrary.MultiplyMultiply_FloatFloat` (- 1.0 _alpha) 2.0))
      (`SpotLightComponent.SetOuterConeAngle` (`self.SpotLight`) (`KismetMathLibrary.Lerp` 60.0 0.0 _returnvalue_2))
      (`SpotLightComponent.SetOuterConeAngle` (`self.SpotLight1`) (`KismetMathLibrary.Lerp` 60.0 0.0 _returnvalue_2))
      (`SpotLightComponent.SetOuterConeAngle` (`self.SpotLight2`) (`KismetMathLibrary.Lerp` 60.0 0.0 _returnvalue_2))
      (`AudioComponent.SetVolumeMultiplier` _returnvalue (`KismetMathLibrary.Lerp` 2.5 0.0 _returnvalue_2)))))

(event `Toggle`
  (`/Engine/EditorBlueprintResources/StandardMacros.FlipFlop`
    (:`A`
      (`GameplayStatics.PlaySoundAtLocation` "/Game/Sound/SW_Open.SW_Open" (`self.K2_GetActorLocation`) (struct) 1.0 1.0 0.0 null null null null)
      (bind (_direction _alpha) (`Timeline|Timeline` :!label _label)
        (:`Update`
          (`SceneComponent.K2_SetRelativeRotation` (`self.WashingMachine_xyj_gaizi`) (`KismetMathLibrary.RLerp` (struct :`Yaw` 20.0) (struct) (`KismetMathLibrary.MultiplyMultiply_FloatFloat` (- 1.0 _alpha) 4.0) true) false false)
          (switch `ETimelineDirection` _direction
            (:`Backward`
              (`LightComponent.SetIntensity` (`self.PointLight1`) (`KismetMathLibrary.Lerp` 0.0 2.0 _alpha)))))))
    (:`B`
      (`GameplayStatics.PlaySoundAtLocation` "/Game/Sound/SW_Close.SW_Close" (`self.K2_GetActorLocation`) (struct) 1.0 1.0 0.0 null null null null)
      (goto _label :!via `Reverse`))))

(fn `UserConstructionScript`)