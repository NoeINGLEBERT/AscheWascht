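; BP_Curtain is a scale-animated curtain with lights that stages game flow, from player start through towel waves to the ending.
; Timelines drive curtain and light transitions; interacting opens it and toggles the washing machine.
; Reset polls each frame until it is out of sight and the player is past it, then restores it and spawns the next wave.
; After REDLIGHT, a player overlap closes it, swaps the set for a final washing machine and reopens.
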(event `REDLIGHT`
  (bind (_direction _newtrack_0) (`Timeline|Timeline_1` :!via `PlayFromStart`)
    (:`Update`
      (bind _returnvalue (`KismetMathLibrary.MultiplyMultiply_FloatFloat` (- 1.0 _newtrack_0) 2.0))
      (`SpotLightComponent.SetOuterConeAngle` (`self.SpotLight`) (`KismetMathLibrary.Lerp` 60.0 0.0 _returnvalue))
      (`LightComponent.SetIntensity` (`self.SpotLight1`) (`KismetMathLibrary.Lerp` 0.0 7.0 _returnvalue)))
    (:`Finished`
      (set `self.RED` true))))

(event `GAME OVER`
  (bind (_direction _newtrack_0) (`Timeline|TimelineEnd`)
    (:`Update`
      (`LightComponent.SetIntensity` (`self.RectLight`) (`KismetMathLibrary.Lerp` 1.0 0.05 _newtrack_0))
      (`LightComponent.SetIntensity` (`self.RectLight1`) (`KismetMathLibrary.Lerp` 0.1 0.005 _newtrack_0)))
    (:`Finished`
      (bind (_direction_2 _newtrack_0_2) (`Timeline|Timeline_0`)
        (:`Update`
          (`LightComponent.SetIntensity` (`self.SpotLight1`) (`KismetMathLibrary.Lerp` 0.0 7.0 _newtrack_0_2)))))))

(event `/Game/FirstPerson/Blueprints/BPI_Interact.InteractedWith`
  (params (Player :type "/Game/FirstPerson/Blueprints/BP_FirstPersonCharacter Object Reference"))
  (if (== (`SpotLightComponent.OuterConeAngle` (`self.SpotLight`)) 60.0)
    (`|ExecutionSequence`
      (:`then_0`
        (bind (_direction _alpha) (`Timeline|Open` :!via `PlayFromStart` :!label _label)
          (:`Update`
            (bind _returnvalue (- 1.0 _alpha))
            (`self.SetActorScale3D` (`KismetMathLibrary.VLerp` (1.6 0.5 1.0) (1.6 2.5 1.0) (`KismetMathLibrary.MultiplyMultiply_FloatFloat` _returnvalue 4.0)))
            (if (not (`self.RED`))
              (bind _returnvalue_2 (`KismetMathLibrary.MultiplyMultiply_FloatFloat` _returnvalue 2.0))
              (`SpotLightComponent.SetOuterConeAngle` (`self.SpotLight`) (`KismetMathLibrary.Lerp` 0.0 60.0 _returnvalue_2))
              (`LightComponent.SetIntensity` (`self.RectLight`) (`KismetMathLibrary.Lerp` 1.0 0.25 _returnvalue_2))
              (`LightComponent.SetIntensity` (`self.RectLight1`) (`KismetMathLibrary.Lerp` 0.1 0.025 _returnvalue_2))))))
      (:`then_1`
        (bind _returnvalue_3 (`GameplayStatics.GetActorOfClass` "/Game/WashingMachine/BP_WashingMachine.BP_WashingMachine_C"))
        (`/Game/WashingMachine/BP_WashingMachine.Toggle` _returnvalue_3)))))

(event `OpenEnd`
  (goto _label))

(event `Close`
  (goto _label :!via `Reverse`))

(event `Reset`
  (bind _returnvalue_x (`KismetMathLibrary.BreakVector` (`self.K2_GetActorLocation`)))
  (bind _bpc_visible (`self.BPC_Visible`))
  (bind _returnvalue_x_2 (`KismetMathLibrary.BreakVector` (`self.K2_GetActorLocation` (`/Game/BPC_Visible.Player` _bpc_visible))))
  (if (and (`/Game/BPC_Visible.OutOfSight` _bpc_visible) (> _returnvalue_x_2 (+ _returnvalue_x 75.0))) :!label _label_2
    (`self.SetActorScale3D` (1.6 2.5 1.0))
    (`SpotLightComponent.SetOuterConeAngle` (`self.SpotLight`) 0.0)
    (bind _returnvalue (`GameplayStatics.GetActorOfClass` "/Game/Towel/BP_TowelSpawner.BP_TowelSpawner_C"))
    (bind _result (`/Engine/EditorBlueprintResources/StandardMacros.IncrementInt` (`/Game/Towel/BP_TowelSpawner.WaveIndex` _returnvalue))
      (:`  `
        (`/Game/Towel/BP_TowelSpawner.SpawnTowels` _returnvalue _result)))
    (else
      (`KismetSystemLibrary.Delay` 0.0)
      (goto _label_2))))

(event `Start`
  (bind (_direction _alpha) (`Timeline|Timeline` :!via `PlayFromStart`)
    (:`Update`
      (bind _returnvalue (`KismetMathLibrary.MultiplyMultiply_FloatFloat` (- 1.0 _alpha) 2.0))
      (`SpotLightComponent.SetOuterConeAngle` (`self.SpotLight`) (`KismetMathLibrary.Lerp` 60.0 0.0 _returnvalue))
      (`LightComponent.SetIntensity` (`self.RectLight`) (`KismetMathLibrary.Lerp` 0.25 1.0 _returnvalue))
      (`LightComponent.SetIntensity` (`self.RectLight1`) (`KismetMathLibrary.Lerp` 0.025 0.1 _returnvalue)))
    (:`Finished`
      (bind _returnvalue_2 (`GameplayStatics.GetActorOfClass` "/Game/FirstPerson/Blueprints/BP_FirstPersonCharacter.BP_FirstPersonCharacter_C"))
      (`/Game/FirstPerson/Blueprints/BP_FirstPersonCharacter.Begin` _returnvalue_2))))

(event `self.Box1.OnComponentBeginOverlap`
  (params (OverlappedComponent :type "PrimitiveComponent Object Reference") (OtherActor :type "Actor Object Reference") (OtherComp :type "PrimitiveComponent Object Reference") (OtherBodyIndex :type Integer) (bFromSweep :type Boolean) (SweepResult :type "HitResult Structure (by ref)"))
  (cast `/Game/FirstPerson/Blueprints/BP_FirstPersonCharacter` OtherActor)
  (if (`self.RED`)
    (`/Engine/EditorBlueprintResources/StandardMacros.DoOnce` false
      (:`Completed`
        (`self.Close`)
        (`KismetSystemLibrary.Delay` 3.0)
        (bind _returnvalue (`GameplayStatics.GetActorOfClass` "/Game/WashingMachine/BP_WashingMachine.BP_WashingMachine_C"))
        (`self.K2_DestroyActor` _returnvalue)
        (bind _returnvalue_2 (`GameplayStatics.GetActorOfClass` "/Game/BP_Locker.BP_Locker_C"))
        (`self.K2_DestroyActor` _returnvalue_2)
        (bind _returnvalue_3 (`GameplayStatics.GetActorOfClass` "/Game/BP_Wall.BP_Wall_C"))
        (`self.K2_DestroyActor` _returnvalue_3)
        (bind _returnvalue_4 (`|SpawnActorFromClass` "/Game/WashingMachine/BP_WashingMachineFinal.BP_WashingMachineFinal_C" (`KismetMathLibrary.MakeTransform` (265.0 0.0 -52.5) (struct :`Yaw` 90.0) (-2.3 2.3 2.3)) "Undefined" "MultiplyWithRoot" null null))
        (`KismetSystemLibrary.Delay` 3.0)
        (`self.OpenEnd`)
        (`KismetSystemLibrary.Delay` 1.0)
        (`/Game/WashingMachine/BP_WashingMachineFinal.Toggle` _returnvalue_4)))))

(fn `UserConstructionScript`)