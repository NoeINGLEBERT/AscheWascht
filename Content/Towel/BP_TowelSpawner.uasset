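; BP_TowelSpawner is an actor that spawns BP_Towel actors with random rotations across an area marked by three arrow components.
; SpawnTowels runs a nested loop up to LastIndex, interpolating positions along Arrow-to-Arrow1 and Arrow-to-Arrow2 to form a parallelogram grid.
; BeginPlay passes a LastIndex of zero, so it spawns a single towel and the interpolation divides by zero.
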(event `self.ReceiveBeginPlay`
  (`self.SpawnTowels` 0))

(event `SpawnTowels`
  (params (LastIndex :type Integer))
  (bind _returnvalue (`SceneComponent.K2_GetComponentLocation` (`self.Arrow`)))
  (for _index (range (+ LastIndex 1))
    (for _index_2 (range (+ LastIndex 1))
      (`|SpawnActorFromClass` "/Game/Towel/BP_Towel.BP_Towel_C" (`KismetMathLibrary.MakeTransform` (+ _returnvalue (* (/ (`KismetMathLibrary.Conv_IntToDouble` _index) (`KismetMathLibrary.Conv_IntToDouble` LastIndex)) (- (`SceneComponent.K2_GetComponentLocation` (`self.Arrow1`)) _returnvalue)) (* (/ (`KismetMathLibrary.Conv_IntToDouble` _index_2) (`KismetMathLibrary.Conv_IntToDouble` LastIndex)) (- (`SceneComponent.K2_GetComponentLocation` (`self.Arrow2`)) _returnvalue))) (`KismetMathLibrary.RandomRotator` true)) "Undefined" "MultiplyWithRoot" null null))))

(fn `UserConstructionScript`)