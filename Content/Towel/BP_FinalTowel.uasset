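; BP_FinalTowel is an interactable towel that the player can pick up, which triggers the curtain's red-light event.
; On interaction, if the player's GrabbedActor check passes, it registers itself as the grabbed actor, plays a grab sound and disables physics and collision.
; It attaches to the player's spring arm, moves in front of the first-person camera keeping its rotation, then calls REDLIGHT on BP_Curtain.
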(event `self.InteractedWith`
  (params (Player :type "/Game/FirstPerson/Blueprints/BP_FirstPersonCharacter Object Reference"))
  (bind _firstpersoncamera (`/Game/FirstPerson/Blueprints/BP_FirstPersonCharacter.FirstPersonCamera` Player))
  (bind _towel (`self.Towel`))
  (if (== (`/Game/FirstPerson/Blueprints/BP_FirstPersonCharacter.GrabbedActor` Player) null)
    (set `/Game/FirstPerson/Blueprints/BP_FirstPersonCharacter.GrabbedActor` self Player)
    (`GameplayStatics.PlaySoundAtLocation` "/Game/Sound/SW_TowelGrab.SW_TowelGrab" (`self.K2_GetActorLocation`) (struct) 1.0 1.0 0.0 null null null null)
    (`PrimitiveComponent.SetSimulatePhysics` _towel false)
    (`PrimitiveComponent.SetCollisionEnabled` _towel "NoCollision")
    (set `self.TempRot` (`self.K2_GetActorRotation`))
    (`self.K2_AttachToComponent` (`/Game/FirstPerson/Blueprints/BP_FirstPersonCharacter.SpringArm` Player) "None" "KeepRelative" "KeepRelative" "KeepRelative" false)
    (`self.K2_SetActorLocationAndRotation` (+ (`SceneComponent.K2_GetComponentLocation` _firstpersoncamera) (* (`SceneComponent.GetForwardVector` _firstpersoncamera) 100.0)) (`self.TempRot`))
    (bind _returnvalue (`GameplayStatics.GetActorOfClass` "/Game/Curtain/BP_Curtain.BP_Curtain_C"))
    (`/Game/Curtain/BP_Curtain.REDLIGHT` _returnvalue)))

(fn `UserConstructionScript`)