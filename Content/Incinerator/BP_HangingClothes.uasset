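; BP_HangingClothes is a clothesline prop that hangs three static meshes along a cable component.
; The construction script places them at fixed cable particles, gives each a random yaw, and rolls three random particle indices near those points.
; Tick moves each mesh to the cable particle at its rolled index, so the clothes follow the simulated cable's motion.
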(event `self.ReceiveTick`
  (params (DeltaSeconds :type "Float (single-precision)"))
  (bind _locations (`CableComponent.GetCableParticleLocations` (`self.Cable`)))
  (`SceneComponent.K2_SetWorldLocation` (`self.StaticMesh`) (`|GetArrayItem` _locations (`self.1`)) false false)
  (`SceneComponent.K2_SetWorldLocation` (`self.StaticMesh1`) (`|GetArrayItem` _locations (`self.2`)) false false)
  (`SceneComponent.K2_SetWorldLocation` (`self.StaticMesh2`) (`|GetArrayItem` _locations (`self.3`)) false false))

(fn `UserConstructionScript`
  (bind _locations (`CableComponent.GetCableParticleLocations` (`self.Cable`)))
  (set `self.1` (`KismetMathLibrary.RandomIntegerInRange` 4 6))
  (set `self.2` (`KismetMathLibrary.RandomIntegerInRange` 9 11))
  (set `self.3` (`KismetMathLibrary.RandomIntegerInRange` 14 16))
  (`SceneComponent.K2_SetWorldLocation` (`self.StaticMesh`) (`|GetArrayItem` _locations 5) false false)
  (`SceneComponent.K2_SetWorldLocation` (`self.StaticMesh1`) (`|GetArrayItem` _locations 10) false false)
  (`SceneComponent.K2_SetWorldLocation` (`self.StaticMesh2`) (`|GetArrayItem` _locations 15) false false)
  (`SceneComponent.K2_SetWorldRotation` (`self.StaticMesh`) (`KismetMathLibrary.MakeRotator` 0.0 0.0 (`KismetMathLibrary.RandomFloatInRange` 0.0 360.0)) false false)
  (`SceneComponent.K2_SetWorldRotation` (`self.StaticMesh1`) (`KismetMathLibrary.MakeRotator` 0.0 0.0 (`KismetMathLibrary.RandomFloatInRange` 0.0 360.0)) false false)
  (`SceneComponent.K2_SetWorldRotation` (`self.StaticMesh2`) (`KismetMathLibrary.MakeRotator` 0.0 0.0 (`KismetMathLibrary.RandomFloatInRange` 0.0 360.0)) false false))