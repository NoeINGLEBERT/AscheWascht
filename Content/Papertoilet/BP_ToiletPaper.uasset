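; A toilet paper pickup that reveals itself, can be grabbed by the player, and triggers the curtain when used again.
; From BeginPlay a zero-delay loop polls until BP_Curtain reaches a set Y scale and BPCVisible reports out of sight, then lights the spotlight and shows the holder.
; Interacting attaches it to the player's spring arm while a timeline fades the light.
; Interacting again starts the curtain and destroys the actor.
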(event `self.ReceiveBeginPlay`
  (bind _returnvalue (`GameplayStatics.GetActorOfClass` "/Game/Curtain/BP_Curtain.BP_Curtain_C"))
  (bind _output_get (set `self.Curtain` _returnvalue))
  (bind (_returnvalue_x _returnvalue_y) (`KismetMathLibrary.BreakVector` (`self.GetActorScale3D` _output_get)))
  (if (and (== _returnvalue_y 2.5) (`/Game/BPC_Visible.OutOfSight` (`self.BPC_Visible`))) :!label _label
    (`LightComponent.SetIntensity` (`self.SpotLight`) 1.0)
    (`SceneComponent.SetVisibility` (`self.Toilet_Paper__Holder_Cylinder_1`) true false)
    (else
      (`KismetSystemLibrary.Delay` 0.0)
      (goto _label))))

(event `/Game/FirstPerson/Blueprints/BPI_Interact.InteractedWith`
  (params (Player :type "/Game/FirstPerson/Blueprints/BP_FirstPersonCharacter Object Reference"))
  (bind _grabbedactor (`/Game/FirstPerson/Blueprints/BP_FirstPersonCharacter.GrabbedActor` Player))
  (if (`SceneComponent.bVisible` (`self.Toilet_Paper__Holder_Cylinder_1`))
    (if (== _grabbedactor null)
      (set `/Game/FirstPerson/Blueprints/BP_FirstPersonCharacter.GrabbedActor` self Player)
      (`|ExecutionSequence`
        (:`then_0`
          (set `self.TempRot` (`self.K2_GetActorRotation`))
          (`self.K2_AttachToComponent` (`/Game/FirstPerson/Blueprints/BP_FirstPersonCharacter.SpringArm` Player) "None" "KeepRelative" "KeepRelative" "KeepRelative" false)
          (`self.K2_SetActorRelativeRotation` (struct))
          (`self.K2_SetActorRelativeLocation` (-75.0 0.0 0.0)))
        (:`then_1`
          (bind (_direction _alpha) (`Timeline|Timeline`)
            (:`Update`
              (`LightComponent.SetIntensity` (`self.SpotLight`) (`KismetMathLibrary.Lerp` 1.0 0.0 _alpha))))))
      (elif (== _grabbedactor self)
        (set `/Game/FirstPerson/Blueprints/BP_FirstPersonCharacter.GrabbedActor` null Player)
        (bind _returnvalue (`GameplayStatics.GetActorOfClass` "/Game/Curtain/BP_Curtain.BP_Curtain_C"))
        (`/Game/Curtain/BP_Curtain.Start` _returnvalue)
        (`self.K2_DestroyActor`)))))

(fn `UserConstructionScript`)